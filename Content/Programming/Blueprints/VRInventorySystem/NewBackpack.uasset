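; A VR inventory backpack that stays hidden until a motion controller grabs it.
; Grab snaps it to the controller, shows the mesh with shadow casting and flags it active.
; Release from that same controller clears the reference and, if a default component is valid, snaps it back there, hides it and clears the flag.
; The Active function exposes that state.
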(event `/Game/Programming/Blueprints/Interfaces/GrabInterface.Grab`
  (params (MotionController :type "MotionControllerComponent Object Reference"))
  (bind _output_get (set `self.Motion Controller` MotionController))
  (`self.K2_AttachToComponent` _output_get "None" "SnapToTarget" "SnapToTarget" "KeepWorld")
  (`SceneComponent.SetHiddenInGame` (`self.StaticMesh`) false true)
  (`PrimitiveComponent.SetCastShadow` (`self.StaticMesh`) true)
  (set `self.Activated?` true))

(event `/Game/Programming/Blueprints/Interfaces/GrabInterface.Release`
  (params (MotionController :type "MotionControllerComponent Object Reference"))
  (if (== MotionController (`self.Motion Controller`))
    (set `self.Motion Controller` null)
    (bind _defaultcomponent (`self.DefaultComponent`)
      (:`then`
        (`self.K2_AttachToComponent` _defaultcomponent "None" "SnapToTarget" "SnapToTarget" "KeepWorld")
        (`SceneComponent.SetHiddenInGame` (`self.StaticMesh`) true true)
        (`PrimitiveComponent.SetCastShadow` (`self.StaticMesh`) false)
        (set `self.Activated?` false))
      (:`else`))))

(fn `Active`
  (returns (`IsActive?` :type Boolean))
  (return (`self.Activated?`)))

(fn `UserConstructionScript`
  (`SceneComponent.SetHiddenInGame` (`self.StaticMesh`) true true))