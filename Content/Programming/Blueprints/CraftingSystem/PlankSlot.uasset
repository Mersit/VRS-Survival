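; PlankSlot is a crafting-system slot actor that detects when the player's held board is positioned across it for placement.
; Left and right collision volumes set check flags when the character's CurrentPlaceableObject overlaps them, with only the right also requiring it to match ItemBoard.
; Each qualifying begin overlap sets the character's BoardPlaceable to whether both flags are true.
; End overlaps never update BoardPlaceable, and the right one sets RightCheck true instead of clearing it.
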(event `self.LeftSideCollision.OnComponentBeginOverlap`
  (params (OverlappedComponent :type "PrimitiveComponent Object Reference") (OtherActor :type "Actor Object Reference") (OtherComp :type "PrimitiveComponent Object Reference") (OtherBodyIndex :type Integer) (bFromSweep :type Boolean) (SweepResult :type "HitResult Structure (by ref)"))
  (if (== OtherActor (`/Game/Programming/Blueprints/Character/FirstPersonCharacter.CurrentPlaceableObject` (cast `/Game/Programming/Blueprints/Character/FirstPersonCharacter` (`GameplayStatics.GetPlayerCharacter` 0) :!pure true)))
    (set `self.LeftCheck?` true)
    (if (and (`self.LeftCheck?`) (`self.RightCheck?`))
      (bind _asfirst_person_character (cast `/Game/Programming/Blueprints/Character/FirstPersonCharacter` (`GameplayStatics.GetPlayerCharacter` 0)))
      (set `/Game/Programming/Blueprints/Character/FirstPersonCharacter.BoardPlaceable?` true _asfirst_person_character)
      (else
        (bind _asfirst_person_character_2 (cast `/Game/Programming/Blueprints/Character/FirstPersonCharacter` (`GameplayStatics.GetPlayerCharacter` 0)))
        (set `/Game/Programming/Blueprints/Character/FirstPersonCharacter.BoardPlaceable?` false _asfirst_person_character_2)))))

(event `self.LeftSideCollision.OnComponentEndOverlap`
  (params (OverlappedComponent :type "PrimitiveComponent Object Reference") (OtherActor :type "Actor Object Reference") (OtherComp :type "PrimitiveComponent Object Reference") (OtherBodyIndex :type Integer))
  (if (== OtherActor (`/Game/Programming/Blueprints/Character/FirstPersonCharacter.CurrentPlaceableObject` (cast `/Game/Programming/Blueprints/Character/FirstPersonCharacter` (`GameplayStatics.GetPlayerCharacter` 0) :!pure true)))
    (set `self.LeftCheck?` false)))

(event `self.RightSideCollision.OnComponentBeginOverlap`
  (params (OverlappedComponent :type "PrimitiveComponent Object Reference") (OtherActor :type "Actor Object Reference") (OtherComp :type "PrimitiveComponent Object Reference") (OtherBodyIndex :type Integer) (bFromSweep :type Boolean) (SweepResult :type "HitResult Structure (by ref)"))
  (bind _currentplaceableobject (`/Game/Programming/Blueprints/Character/FirstPersonCharacter.CurrentPlaceableObject` (cast `/Game/Programming/Blueprints/Character/FirstPersonCharacter` (`GameplayStatics.GetPlayerCharacter` 0) :!pure true)))
  (if (and (== OtherActor _currentplaceableobject) (== _currentplaceableobject "/Game/Programming/Blueprints/InventorySystem/Items/ItemBoard.ItemBoard"))
    (set `self.RightCheck?` true)
    (if (and (`self.LeftCheck?`) (`self.RightCheck?`))
      (bind _asfirst_person_character (cast `/Game/Programming/Blueprints/Character/FirstPersonCharacter` (`GameplayStatics.GetPlayerCharacter` 0)))
      (set `/Game/Programming/Blueprints/Character/FirstPersonCharacter.BoardPlaceable?` true _asfirst_person_character)
      (else
        (bind _asfirst_person_character_2 (cast `/Game/Programming/Blueprints/Character/FirstPersonCharacter` (`GameplayStatics.GetPlayerCharacter` 0)))
        (set `/Game/Programming/Blueprints/Character/FirstPersonCharacter.BoardPlaceable?` false _asfirst_person_character_2)))))

(event `self.RightSideCollision.OnComponentEndOverlap`
  (params (OverlappedComponent :type "PrimitiveComponent Object Reference") (OtherActor :type "Actor Object Reference") (OtherComp :type "PrimitiveComponent Object Reference") (OtherBodyIndex :type Integer))
  (if (== OtherActor (`/Game/Programming/Blueprints/Character/FirstPersonCharacter.CurrentPlaceableObject` (cast `/Game/Programming/Blueprints/Character/FirstPersonCharacter` (`GameplayStatics.GetPlayerCharacter` 0) :!pure true)))
    (set `self.RightCheck?` true)))

(fn `UserConstructionScript`)