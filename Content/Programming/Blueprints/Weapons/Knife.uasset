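; Knife weapon Blueprint, a child weapon that reuses the gun framework with a single-round clip and its own gun type, set in the construction script.
; StartShooting passes through a gate and, if ammo remains, spends a round, plays the Gun animation unless the player is reloading, then calls LineTrace.
; LineTrace is empty: its sphere trace, impact emitter and damage nodes are disconnected, so the knife deals no damage here.
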(event `self.StartShooting`
  (`|ExecutionSequence`
    (:`then_0`
      (goto _label :!via `Open`))
    (:`then_1`
      (`/Engine/EditorBlueprintResources/StandardMacros.Gate` true :!label _label
        (:`Exit`
          (`|ExecutionSequence`
            (:`then_0`
              (if (> (`self.AmmoCurrent`) 0)
                (`self.AmmoCheck`)
                (`self.LineTrace`)
                (`KismetSystemLibrary.Delay` 2.0)))))))))

(event `self.StopShooting`
  (goto _label :!via `Close`))

(fn `AmmoCheck`
  ;[1 1 1] Removes a bullet from ammo everytime a shot is fired, then plays an animation so long as the gun is not reloading
  (`/Engine/EditorBlueprintResources/StandardMacros.DecrementInt` (`self.AmmoCurrent`)
    (:`  `
      (if (not (`/Game/Programming/Blueprints/Character/FirstPersonCharacter.IsReloading?` (cast `/Game/Programming/Blueprints/Character/FirstPersonCharacter` (`GameplayStatics.GetPlayerCharacter` 0) :!pure true)))
        (`SkeletalMeshComponent.PlayAnimation` (`self.Gun`) null false)))))

(fn `LineTrace`
  ;[1 1 1] Fires a line trace from the camera and the gun barrel, then plays an emitter at impact location and deals damage to enemy if they are hit
)

(fn `UserConstructionScript`
  ;[1 1 1] Sets the default values for the weapon
  (`parent.UserConstructionScript`)
  (set `self.AmmoMax` 30)
  (set `self.AmmoCurrent` 1)
  (set `self.ClipSize` 1)
  (set `self.ReloadSpeed` 3.0)
  (set `self.BulletSpread` 0.0)
  (set `self.GunType` "NewEnumerator9"))