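; WeaponParent is a base weapon Blueprint that declares empty events for reload, equip, unequip and start/stop shooting.
; Its construction script snaps the Gun component to a GripPoint socket, intended as the player's hand attachment.
; ReloadGun fills the clip from reserve ammo and plays a gun-type-specific sound at the barrel.
; When reserves fall short, it loads the remainder and plays no sound.
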(event `Reload`
  ;[1 1 1] Holds the custom events for the weapons
)

(event `Equip`
  ;[1 1 1] Holds the custom events for the weapons
)

(event `StartShooting`
  ;[1 1 1] Holds the custom events for the weapons
)

(event `Unequip`
  ;[1 1 1] Holds the custom events for the weapons
)

(event `StopShooting`
  ;[1 1 1] Holds the custom events for the weapons
)

(fn `Reload Gun`
  ;[1 1 1] Reloads Gun Function
  (bind _output_get (set `self.BulletDifference` (- (`self.ClipSize`) (`self.AmmoCurrent`))))
  (if (>= (`self.AmmoMax`) _output_get)
    (set `self.AmmoCurrent` (`self.ClipSize`))
    (set `self.AmmoMax` (- (`self.AmmoMax`) (`self.BulletDifference`)))
    (if (`|EnumEquality` (`self.GunType`) "NewEnumerator5")
      (`GameplayStatics.PlaySoundAtLocation` "/Game/Programming/Sounds/repeaterreload.repeaterreload" (`SceneComponent.K2_GetComponentLocation` (`self.BarrelRef`)) (struct) 1.0 1.0 0.0 null null null null)
      (elif (`|EnumEquality` (`self.GunType`) "NewEnumerator6")
        (`GameplayStatics.PlaySoundAtLocation` "/Game/Programming/Sounds/revolverreload.revolverreload" (`SceneComponent.K2_GetComponentLocation` (`self.BarrelRef`)) (struct) 1.0 1.0 0.0 null null null null)
        (elif (`|EnumEquality` (`self.GunType`) "NewEnumerator7")
          (`GameplayStatics.PlaySoundAtLocation` "/Game/Programming/Sounds/shotgunreload.shotgunreload" (`SceneComponent.K2_GetComponentLocation` (`self.BarrelRef`)) (struct) 1.0 1.0 0.0 null null null null)
          (elif (`|EnumEquality` (`self.GunType`) "NewEnumerator8")
            (`GameplayStatics.PlaySoundAtLocation` "/Game/Programming/Sounds/sniperreload.sniperreload" (`SceneComponent.K2_GetComponentLocation` (`self.BarrelRef`)) (struct) 1.0 1.0 0.0 null null null null)))))
    (else
      (set `self.AmmoCurrent` (+ (`self.AmmoMax`) (`self.AmmoCurrent`)))
      (set `self.AmmoMax` 0))))

(fn `UserConstructionScript`
  ;[1 1 1] Attaches weapon to players hands
  (`SceneComponent.K2_AttachToComponent` (`self.Gun`) null "GripPoint" "SnapToTarget" "SnapToTarget" "SnapToTarget" true))