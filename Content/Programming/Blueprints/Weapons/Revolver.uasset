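; Revolver weapon Blueprint that sets its ammo, reload and spread defaults on construction and writes its name to the FirstPersonCharacter.
; StartShooting passes through a gate and, with ammo left, decrements it, animates unless reloading, then fires.
; LineTrace plays muzzle effects and sphere-traces from the barrel with random world X/Y spread, spawning an impact emitter.
; Damage logic is disconnected, and CanFire is set after a delay but never checked here.
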(event `self.StartShooting`
  (`|ExecutionSequence`
    (:`then_0`
      (goto _label :!via `Open`))
    (:`then_1`
      (`/Engine/EditorBlueprintResources/StandardMacros.Gate` true :!label _label
        (:`Exit`
          (`|ExecutionSequence`
            (:`then_0`
              (if (> (`self.AmmoCurrent`) 0)
                (`self.AmmoCheck`)
                (`self.LineTrace`)
                (`KismetSystemLibrary.Delay` 5.0)
                (set `self.CanFire?` true)))))))))

(event `self.StopShooting`
  (goto _label :!via `Close`))

(fn `AmmoCheck`
  ;[1 1 1] Removes a bullet from ammo everytime a shot is fired, then plays an animation so long as the gun is not reloading
  (`/Engine/EditorBlueprintResources/StandardMacros.DecrementInt` (`self.AmmoCurrent`)
    (:`  `
      (if (not (`/Game/Programming/Blueprints/Character/FirstPersonCharacter.IsReloading?` (cast `/Game/Programming/Blueprints/Character/FirstPersonCharacter` (`GameplayStatics.GetPlayerCharacter` 0) :!pure true)))
        (`SkeletalMeshComponent.PlayAnimation` (`self.Gun`) null false)))))

(fn `LineTrace`
  (bind _bulletspread (`self.BulletSpread`))
  (bind _returnvalue (`SceneComponent.K2_GetComponentLocation` (`self.BarrelRef`)))
  (bind _returnvalue_2 (`SceneComponent.K2_GetComponentLocation` (`self.BarrelRef`)))
  (bind _returnvalue_3 (* _bulletspread -1.0))
  ;[1 1 1] Fires a line trace from the camera and the gun barrel, then plays an emitter at impact location and deals damage to enemy if they are hit
  (`GameplayStatics.SpawnEmitterAtLocation` null _returnvalue)
  (`GameplayStatics.PlaySoundAtLocation` "/Game/Programming/Sounds/revolvershoot.revolvershoot" _returnvalue (struct) 1.0 1.0 0.0 null null null null)
  (bind _outhit (`KismetSystemLibrary.SphereTraceSingle` _returnvalue_2 (+ (+ _returnvalue_2 (* (`SceneComponent.GetForwardVector` (`self.Arrow`)) (`self.Range`))) (`KismetMathLibrary.MakeVector` (`KismetMathLibrary.RandomFloatInRange` _returnvalue_3 _bulletspread) (`KismetMathLibrary.RandomFloatInRange` _returnvalue_3 _bulletspread))) 4.0 "TraceTypeQuery1"))
  (`GameplayStatics.SpawnEmitterAtLocation` null (`.ImpactPoint` (`GameplayStatics.BreakHitResult` _outhit))))

(fn `UserConstructionScript`
  ;[1 1 1] Sets the default values for the weapon
  (`parent.UserConstructionScript`)
  (set `self.AmmoMax` 120)
  (set `self.AmmoCurrent` 6)
  (set `self.ClipSize` 6)
  (set `self.ReloadSpeed` 3.0)
  (set `self.BulletSpread` 300.0)
  (set `self.GunType` "NewEnumerator6")
  (bind _returnvalue (`GameplayStatics.GetActorOfClass` "/Game/Programming/Blueprints/Character/FirstPersonCharacter.FirstPersonCharacter_C"))
  (set `/Game/Programming/Blueprints/Character/FirstPersonCharacter.WeaponName` "Revolver" _returnvalue))