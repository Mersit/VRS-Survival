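; BP_Cultist is an enemy for a VR game that registers itself in VRGameMode's living-enemy count on BeginPlay.
; Its capsule applies fixed damage to any actor that begins overlapping it.
; DealDamage sets Health to Damage minus Health, an apparently reversed subtraction.
; At zero or below, it decrements the enemy count, has the game mode check for remaining enemies and destroys itself.
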(event `self.ReceiveBeginPlay`
  (bind _asvrgame_mode (cast `/Game/VRTemplate/Blueprints/VRGameMode` (`GameplayStatics.GetGameMode`)))
  (`/Engine/EditorBlueprintResources/StandardMacros.IncrementInt` (`/Game/VRTemplate/Blueprints/VRGameMode.EnemiesAlive` _asvrgame_mode)))

(event `self.Capsule.OnComponentBeginOverlap`
  (params (OverlappedComponent :type "PrimitiveComponent Object Reference") (OtherActor :type "Actor Object Reference") (OtherComp :type "PrimitiveComponent Object Reference") (OtherBodyIndex :type Integer) (bFromSweep :type Boolean) (SweepResult :type "HitResult Structure (by ref)"))
  (bind _returnvalue (`GameplayStatics.ApplyDamage` OtherActor 15.0 null self))
  (`KismetSystemLibrary.PrintString` (`KismetStringLibrary.Conv_DoubleToString` _returnvalue)))

(event `/Game/Interfaces/BPI_Damage.DealDamage`
  (params (Damage :type "Float (double-precision)"))
  (bind _output_get (set `self.Health` (- Damage (`self.Health`))))
  (if (<= _output_get 0.0)
    (`KismetSystemLibrary.PrintString` "Player Died")
    (bind _asvrgame_mode (cast `/Game/VRTemplate/Blueprints/VRGameMode` (`GameplayStatics.GetGameMode`)))
    (`/Engine/EditorBlueprintResources/StandardMacros.DecrementInt` (`/Game/VRTemplate/Blueprints/VRGameMode.EnemiesAlive` _asvrgame_mode)
      (:`  `
        (`/Game/VRTemplate/Blueprints/VRGameMode.CheckEnemyLeft` _asvrgame_mode)
        (`self.K2_DestroyActor`)))
    (else
      (`KismetSystemLibrary.PrintString` (`KismetStringLibrary.Conv_DoubleToString` _output_get)))))

(fn `UserConstructionScript`)